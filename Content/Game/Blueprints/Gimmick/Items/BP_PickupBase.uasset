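; Base Blueprint for interactable item pickups that add their Item to the C++ item manager subsystem.
; When OnlyOnce is set, interacting also executes the EventDestroy component, whose execute event destroys the actor.
; BeginPlay asks that component to check whether the event was already executed.
; GetCommandMessage returns the stored command message for the interacting player.
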(event EDExcuteEvent(Event_Destroy)
  (Actor|DestroyActor))

(event EventBeginPlay
  (Default|CheckEventExcuted (Variables|Default|GetEvent_Destroy)))

(event EventInteract
  (params (Player :type Actor%20Object%20Reference))
  (Class|CPPItemManegerSubsystem|AddItemData (Subsystems|GetCPPItemManegerSubsystem) (Variables|Default|GetItem))
  (if (Variables|Default|GetOnlyOnce)
    (Default|EventExcute (Variables|Default|GetEvent_Destroy))))

(fn ConstructionScript)

(fn GetCommandMessage
  (params (Player :type Actor%20Object%20Reference))
  (return (Variables|Default|GetCommandMassage)))