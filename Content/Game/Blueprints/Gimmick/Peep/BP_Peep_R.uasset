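; Interactable peep gimmick (R variant) that the player can look through and exit.
; Interact sends PeepMessage to the player character, runs CallEDAction, and flip-flops the command prompt between ExitMessage and "覗く" (peep).
; GetCommandMessage returns that prompt.
; CheckPlayerLocation tests which side the player is on, using an offset sign check built from the actor's forward vector and a 45-degree yaw-rotated forward vector.
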(event EventInteract
  (params (Player :type Actor%20Object%20Reference))
  (Class|BPIPlayer|Peep(Message) (Game|GetPlayerCharacter 0) self)
  (Default|CallEDAction)
  (Utilities|FlowControl|FlipFlop
    (:A
      (Variables|Default|SetCommandMessage (Variables|Default|GetExitMessage)))
    (:B
      (Variables|Default|SetCommandMessage "覗く"))))

(fn ConstructionScript)

(fn CheckPlayerLocation
  (bind _returnvalue (Transformation|GetActorRotation))
  (bind _returnvalue_2 (Game|GetPlayerCharacter 0))
  (bind _returnvalue_3 (Transformation|GetActorLocation))
  (bind _returnvalue_4 (Transformation|GetActorLocation _returnvalue_2))
  (bind _returnvalue_5 (Math|Vector|GetForwardVector _returnvalue))
  (bind (_roll _pitch _yaw) (Math|Rotator|BreakRotator _returnvalue))
  (bind (_x _y) (Math|Vector|BreakVector _returnvalue_3))
  (bind (_x_2 _y_2) (Math|Vector|BreakVector _returnvalue_5))
  (bind (_x_3 _y_3) (Math|Vector|BreakVector _returnvalue_4))
  (bind _returnvalue_6 (+ _yaw 45.0))
  (bind _returnvalue_7 (Math|Rotator|MakeRotator _roll _pitch _returnvalue_6))
  (bind _returnvalue_8 (Math|Vector|GetForwardVector _returnvalue_7))
  (bind (_x_4 _y_4) (Math|Vector|BreakVector _returnvalue_8))
  (return (> (* (+ (* (- _y_3 _y) (- _x_2 _y_2)) (* (- _x_3 _x) (+ _x_2 _y_2)) -1e+01) (* _x_4 _y_4)) 0.0)))

(fn GetCommandMessage
  (params (Player :type Actor%20Object%20Reference))
  (return (Variables|Default|GetCommandMessage)))