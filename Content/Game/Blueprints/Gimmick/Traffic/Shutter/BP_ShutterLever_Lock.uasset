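; Interactable shutter lever that stays locked until every lever in its UnlockLevers list is activated.
; On Interact, CheckUnlock scans those levers and, despite its name, returns true while any is still inactive.
; When locked, the command message reads "power is off" in Japanese for a few seconds, then reverts to "move".
; When unlocked, it calls OpenClose on the linked Shutter.
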(event Collision|EventActorBeginOverlap
  (params (OtherActor :type Actor%20Object%20Reference))
  (|CallParentFunction OtherActor) ; This node is disabled and will not be called.\nDrag off pins to build functionality.
)

(event EventTick
  (params (DeltaSeconds :type Float%20%28single-precision%29))
  (|CallParentFunction DeltaSeconds) ; This node is disabled and will not be called.\nDrag off pins to build functionality.
)

(event EventInteract
  (params (Player :type Actor%20Object%20Reference))
  (bind _locked (CallFunction|CheckUnlock))
  (if _locked
    (Variables|Default|SetCommandMassage "電源が切れている")
    (Utilities|FlowControl|Delay 5.0)
    (Variables|Default|SetCommandMassage "動かす")
    (else
      (Default|OpenClose (Variables|Default|GetShutter)))))

(fn ConstructionScript
  (|CallParentFunction))

(fn CheckUnlock
  (Variables|Default|SetLocked false)
  (for _array_element (Variables|Default|GetUnlockLevers)
    (if (not (Variables|/Game/Game/Blueprints/Gimmick/Traffic/Shutter/BP_UnlockLever.BP_UnlockLever_C|GetActivated _array_element))
      (Variables|Default|SetLocked true)))
  (return (Variables|Default|GetLocked)))