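; BP_UnlockLever is an interactable lever gimmick that stays padlocked until unlocked, then can be pulled once.
; LeverUnlock hides the chain and padlock, while GetCommandMessage offers a Japanese unlock prompt when the lever key item is selected.
; Interacting when unlocked fires the EventUnlock component, whose callback marks it activated and rotates the lever on a timeline with sound.
; BeginPlay asks that component to check whether the event was already executed.
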(event EDExcuteEvent(Event_Unlock)
  (Variables|Default|SetActivated true)
  (Audio|PlaySoundatLocation "/Game/Game/Sounds/lever-pushed.lever-pushed" (Transformation|GetActorLocation) "0, 0, 0" 1.0 1.0 0.0 0 0 0 0)
  (bind _newtrack_0 (Timeline|Timeline Play)
    (:Update
      (Transformation|SetRelativeRotation (Variables|Default|GetSM_lever1) (Math|Rotator|Lerp(Rotator) "0, 0, 0" "45.000000,0.000000,0.000000" _newtrack_0) false false))
    (:Finished
      (Variables|Default|SetCommandMassage "起動した"))))

(event EventBeginPlay
  (Default|CheckEventExcuted (Variables|Default|GetEvent_Unlock)))

(event EventInteract
  (params (Player :type Actor%20Object%20Reference))
  (if (Variables|Default|GetUnlocked)
    (if (Variables|Default|GetActivated)
      (Variables|Default|SetCommandMassage "すでに起動されている")
      (else
        (Default|EventExcute (Variables|Default|GetEvent_Unlock))))
    (else
      (Variables|Default|SetCommandMassage "鍵でロックされている"))))

(event EventLeverUnlock
  (Variables|Default|SetUnlocked true)
  (Variables|Default|SetCommandMassage "動かす")
  (Rendering|SetVisibility (Variables|Default|GetSM_Chain) false false)
  (Rendering|SetVisibility (Variables|Default|GetSM_padlock) false false)
  (Audio|PlaySoundatLocation "/Game/Game/Sounds/door-unlock.door-unlock" (Transformation|GetActorLocation) "0, 0, 0" 1.0 1.0 0.0 0 0 0 0))

(fn ConstructionScript)

(fn GetCommandMessage
  (params (Player :type Actor%20Object%20Reference))
  (if (== (Variables|/Script/Black_Shadow.CPP_ItemManegerSubsystem|GetSelectedItemData (Subsystems|GetCPPItemManegerSubsystem)) "/Game/Game/Blueprints/Gimmick/Items/ItemData/DA_Item_LeverKey.DA_Item_LeverKey")
    (if (or (Variables|Default|GetActivated) (Variables|Default|GetUnlocked))
      _
      (else
        (return "E:鍵を開ける"))))
  (return (Variables|Default|GetCommandMassage)))