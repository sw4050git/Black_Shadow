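; BP_Door_GimmickLock is a child door Blueprint whose lock is meant for gimmicks.
; On interact, it shows a Japanese message telling the player to head for the exit while locked, otherwise it opens or closes.
; Its DoorUnlock override runs the parent logic but always returns false.
; BeginPlay and construction just defer to the parent.
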(event EventBeginPlay
  (|CallParentFunction))

(event EventInteract
  (params (Player :type Actor%20Object%20Reference))
  (if (Variables|Default|GetLocked)
    (Variables|Default|SetCommandMessage "今は出口を目指そう…")
    (else
      (CallFunction|OpenClose))))

(fn ConstructionScript
  (|CallParentFunction))

(fn DoorUnlock
  (|CallParentFunction)
  (return false))