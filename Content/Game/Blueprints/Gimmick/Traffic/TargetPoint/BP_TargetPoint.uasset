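; BP_TargetPoint is a waypoint actor in the traffic gimmick that links to other target points to form a directed route graph.
; ConnectLink and CutLink add or remove entries in NextTargetPoints, which is exposed alongside the point's location through getters.
; Given a pawn and controller, it runs synchronous navigation queries to report whether a complete, non-partial path reaches it, and that path's length.
; A debug-arrow drawing of the links is left unconnected.
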(event EventBeginPlay)

(event Collision|EventActorBeginOverlap
  (params (OtherActor :type Actor%20Object%20Reference)))

(event EventTick
  (params (DeltaSeconds :type Float%20%28single-precision%29)))

(event EventConnectLink
  (params (TargetPoint :type Target%20Point%20Object%20Reference))
  (Utilities|Array|AddUnique (Variables|Default|GetNextTargetPoints) TargetPoint))

(event EventCutLink
  (params (TargetPoint :type Target%20Point%20Object%20Reference))
  (Utilities|Array|RemoveItem (Variables|Default|GetNextTargetPoints) TargetPoint))

(fn ConstructionScript)

(fn CheckPathIsAvailable
  (params (Controlled%20Pawn :type Pawn%20Object%20Reference) (Owner%20Controller :type AI%20Controller%20Object%20Reference))
  (bind _returnvalue (Class|NavigationSystemV1|FindPathtoActorSynchronously (Transformation|GetActorLocation Controlled%20Pawn) self 5e+01 Owner%20Controller 0))
  (Utilities|IsValid _returnvalue
    (:Is%20Valid
      (if (not (Class|NavigationPath|IsPartial _returnvalue))
        (return true)
        (else
          _)))
    (:Is%20Not%20Valid
      _))
  (return false))

(fn GetLocation
  (return (Transformation|GetActorLocation)))

(fn GetNextTargetPoints
  (return (Variables|Default|GetNextTargetPoints)))

(fn GetPathDistance
  (params (Controlled%20Pawn :type Pawn%20Object%20Reference) (Owner%20Controller :type AI%20Controller%20Object%20Reference))
  (bind _returnvalue (Class|NavigationSystemV1|FindPathtoActorSynchronously (Transformation|GetActorLocation Controlled%20Pawn) self 5e+01 Owner%20Controller 0))
  (return (Class|NavigationPath|GetPathLength _returnvalue)))