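; BP_TargetLinkController is a traffic gimmick controller that cuts and restores links between pairs of target points.
; Cut and Connect send link messages to both points, so each change applies in both directions.
; CutTargetLink reconnects the previously stored pair, cuts the new pair and stores it, keeping only one link cut at a time through this event.
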(event Custom|Cut
  (params (TargetPoint1 :type Target%20Point%20Object%20Reference) (TargetPoint2 :type Target%20Point%20Object%20Reference))
  (Class|BPITargetPoint|CutLink(Message) TargetPoint1 TargetPoint2)
  (Class|BPITargetPoint|CutLink(Message) TargetPoint2 TargetPoint1))

(event Custom|Connect
  (params (TargetPoint1 :type Target%20Point%20Object%20Reference) (TargetPoint2 :type Target%20Point%20Object%20Reference))
  (Class|BPITargetPoint|ConnectLink(Message) TargetPoint1 TargetPoint2)
  (Class|BPITargetPoint|ConnectLink(Message) TargetPoint2 TargetPoint1))

(event EventBeginPlay)

(event Collision|EventActorBeginOverlap
  (params (OtherActor :type Actor%20Object%20Reference)))

(event EventTick
  (params (DeltaSeconds :type Float%20%28single-precision%29)))

(event EventCutTargetLink
  (params (TargetPoint1 :type Target%20Point%20Object%20Reference) (TargetPoint2 :type Target%20Point%20Object%20Reference))
  (if (Utilities|Array|IsValidIndex (Variables|Default|GetCutTargetPoint) 1)
    (CallFunction|Connect (Utilities|Array|Get(acopy) (Variables|Default|GetCutTargetPoint)) (Utilities|Array|Get(acopy) (Variables|Default|GetCutTargetPoint) 1)))
  (CallFunction|Cut TargetPoint1 TargetPoint2)
  (Variables|Default|SetCutTargetPoint (Utilities|Array|MakeArray TargetPoint1 TargetPoint2)))

(fn ConstructionScript)