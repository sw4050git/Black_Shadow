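; BP_BlockWall is a traffic gimmick blocking wall that supplies a command message when a player queries it.
; An EventChangeMessage component checks on BeginPlay whether its event was already executed, and SetCommandMessage triggers that event.
; When the event fires, CommandMessage switches to ChangedMessage, which GetCommandMessage then returns.
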(event EDExcuteEvent(Event_ChangeMessage)
  (Variables|Default|SetCommandMessage (Variables|Default|GetChangedMessage)))

(event EventBeginPlay
  (Default|CheckEventExcuted (Variables|Default|GetEvent_ChangeMessage)))

(event EventSetCommandMessage
  (params (NewCommandMessage :type Text))
  (Default|EventExcute (Variables|Default|GetEvent_ChangeMessage)))

(fn ConstructionScript)

(fn GetCommandMessage
  (params (Player :type Actor%20Object%20Reference))
  (return (Variables|Default|GetCommandMessage)))