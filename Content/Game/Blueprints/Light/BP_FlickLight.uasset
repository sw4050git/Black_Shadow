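; Flickering lamp actor that pairs a rect light with a lamp mesh and randomizes their blink timing.
; On BeginPlay it creates dynamic instances of the rect light's light function material and the lamp mesh's first material.
; Each receives its own random BlinkTime parameter, so light and mesh timings are not synchronized.
; The blinking itself is left to the materials, with no Tick logic.
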(event EventBeginPlay
  (bind _returnvalue (Math|Random|RandomFloatinRange 0.3 1.0))
  (bind _returnvalue_2 (Rendering|Material|CreateDynamicMaterialInstance (Variables|/Script/Engine.LightComponent|GetLightFunctionMaterial (Variables|Default|GetRectLight)) "None" "None" :!class /Script/Engine.KismetMaterialLibrary))
  (Rendering|Components|Light|SetLightFunctionMaterial (Variables|Default|GetRectLight) _returnvalue_2)
  (Rendering|Material|SetScalarParameterValue _returnvalue_2 "BlinkTime" _returnvalue :!class /Script/Engine.MaterialInstanceDynamic)
  (Rendering|Material|CreateDynamicMaterialInstance (Variables|Default|GetSM_lightinglamp) 0 0 "None" :!class /Script/Engine.PrimitiveComponent)
  (Rendering|Material|SetScalarParameterValueonMaterials (Variables|Default|GetSM_lightinglamp) "BlinkTime" _returnvalue))

(event Collision|EventActorBeginOverlap
  (params (OtherActor :type Actor%20Object%20Reference)))

(event EventTick
  (params (DeltaSeconds :type Float%20%28single-precision%29)))

(fn ConstructionScript)