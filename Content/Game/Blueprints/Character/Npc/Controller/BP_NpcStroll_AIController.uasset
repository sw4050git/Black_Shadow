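; AI controller for a strolling NPC that runs a behavior tree and tracks the player through sight and hearing.
; Perception updates for Player-tagged actors write the heard location to the blackboard, setting the hearing flag only when the navigation path to it is short enough.
; Sight sets the visible flag unless the player has the camera-fixed hide gameplay tag; otherwise a timer clears the flag after a delay.
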(event OnPerceptionUpdated(AIPerception)
  (params (UpdatedActors :type Array%20of%20Actor%20Object%20References))
  (bind _blackboard (Variables|Default|GetBlackboard))
  ;[1 1 1] AIPerception
  (for _array_element UpdatedActors
    (if (Actor|ActorHasTag _array_element "Player")
      (bind _info (Class|AIPerceptionComponent|GetActorsPerception (Variables|Default|GetAIPerception) _array_element))
      (Class|AIController|UseBlackboard "/Game/Game/Blueprints/Character/Npc/AI/BB_NpcBase.BB_NpcBase")
      (bind _returnvalue (Class|NavigationSystemV1|FindPathtoLocationSynchronously (Transformation|GetActorLocation (Pawn|GetControlledPawn)) (.StimulusLocation (Utilities|Struct|BreakAIStimulus (Utilities|Array|Get(acopy) (.LastSensedStimuli (Utilities|Struct|BreakActorPerceptionBlueprintInfo _info)) 1))) 0 0))
      (AI|Components|Blackboard|SetValueasBool _blackboard (Utilities|Name|MakeLiteralName "Flg_Hear") (and (.bSuccessfullySensed (Utilities|Struct|BreakAIStimulus (Utilities|Array|Get(acopy) (.LastSensedStimuli (Utilities|Struct|BreakActorPerceptionBlueprintInfo _info)) 1))) (< (Class|NavigationPath|GetPathLength _returnvalue) 2e+03)))
      (AI|Components|Blackboard|SetValueasVector _blackboard (Utilities|Name|MakeLiteralName "NowDestination") (.StimulusLocation (Utilities|Struct|BreakAIStimulus (Utilities|Array|Get(acopy) (.LastSensedStimuli (Utilities|Struct|BreakActorPerceptionBlueprintInfo _info)) 1))))
      (if (.bSuccessfullySensed (Utilities|Struct|BreakAIStimulus (Utilities|Array|Get(acopy) (.LastSensedStimuli (Utilities|Struct|BreakActorPerceptionBlueprintInfo _info)))))
        (Utilities|IsValid _array_element
          (:Is%20Valid
            (if (not (GameplayTags|HasMatchingGameplayTag (Ability|GetAbilitySystemComponent _array_element) "(TagName=\"Ability.State.CameraFixed.Hide\")"))
              (Utilities|Time|ClearandInvalidateTimerbyHandle (Variables|Default|GetTimer%20))
              (AI|Components|Blackboard|SetValueasBool (Variables|Default|GetBlackboard) (Utilities|Name|MakeLiteralName "Flg_Visible") true)
              (else
                (bind _returnvalue_2 (Utilities|Time|SetTimerbyEvent (delegate Custom|Start%20Timer) (Variables|Default|GetVisible%20Timer) :!label _label))
                (Variables|Default|SetTimer%20 _returnvalue_2))))
          (:Is%20Not%20Valid
            (goto _label)))
        (else
          (goto _label)))))
  (Variables|Default|SetStrength 0.0))

(event Custom|Start%20Timer
  ;[1 1 1] AIPerception
  (AI|Components|Blackboard|SetValueasBool (Variables|Default|GetBlackboard) (Utilities|Name|MakeLiteralName "Flg_Visible") false))

(event EventBeginPlay
  ;[1 1 1] BeginPlay
  (Class|AIController|UseBlackboard (Variables|Default|GetBlackboard%20Asset))
  (AI|Components|Blackboard|SetValueasObject (Variables|Default|GetBlackboard) (Utilities|Name|MakeLiteralName "PlayerActor") (Game|Player|GetPlayerPawn 0))
  (AI|RunBehaviorTree (Variables|Default|GetBTAsset)))

(fn ConstructionScript)