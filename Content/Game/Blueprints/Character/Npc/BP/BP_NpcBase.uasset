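; Base NPC character Blueprint that catches the player on overlap.
; An overlap with a Player-tagged actor that passes IsCatchable stops the NPC's movement and sends the player DeadMessage with the CaughtDirection result.
; UpdateWalkSpeed sets the movement speed, and getters expose a fixed target point and a set of target points.
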(event EventBeginPlay)

(event EventTick
  (params (DeltaSeconds :type Float%20%28single-precision%29)))

(event Collision|EventActorBeginOverlap
  (params (OtherActor :type Actor%20Object%20Reference))
  (if (Actor|ActorHasTag OtherActor "Player")
    (if (|IsCatchable OtherActor)
      (Variables|/Script/Engine.CharacterMovementComponent|SetMaxWalkSpeed (Variables|Character|GetCharacterMovement) 0.0)
      (Class|BPIPlayer|Dead(Message) OtherActor (|CaughtDirection)))))

(event EventUpdateWalkSpeed
  (params (NewWalkSpeed :type Float%20%28double-precision%29))
  (Variables|/Script/Engine.CharacterMovementComponent|SetMaxWalkSpeed (Variables|Character|GetCharacterMovement) NewWalkSpeed))

(fn ConstructionScript)

(fn GetFixTargetPoint
  (return (Variables|Default|GetFixTargetPoint)))

(fn GetTargetPoints
  (return (Variables|Default|GetTargetPoints)))