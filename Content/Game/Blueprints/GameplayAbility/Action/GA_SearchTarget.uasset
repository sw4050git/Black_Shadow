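; GA_SearchTarget is a Gameplay Ability that finds the actor the owner's camera points at and sets it as the owner's target.
; On activation it commits, then line traces along the camera's forward vector for SearchLength on a single trace channel.
; Camera data and the target pass through message calls on the owning actor.
; The hit actor is sent without a hit check, then the ability ends immediately.
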(event Ability|EventActivateAbility
  (Ability|CommitAbility)
  (bind _cameralocation (Class|BPIPlayer|GetCameraLocation(Message) (Ability|GetOwningActorfromActorInfo)))
  (bind _forwardvector (Class|BPIPlayer|GetCameraForwardVector(Message) (Ability|GetOwningActorfromActorInfo)))
  (bind _outhit (Collision|LineTraceByChannel _cameralocation (+ _cameralocation (* _forwardvector (Variables|Default|GetSearchLength))) "TraceTypeQuery3" false 0 "None"))
  (Class|BPIPlayer|SetTargetActor(Message) (Ability|GetOwningActorfromActorInfo) (.HitActor (Collision|BreakHitResult _outhit)))
  (Ability|EndAbility))

(event Ability|EventOnEndAbility
  (params (bWasCancelled :type Boolean)))