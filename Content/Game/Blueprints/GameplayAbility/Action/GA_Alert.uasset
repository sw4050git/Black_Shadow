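; GA_Alert is a gameplay ability that puts its owner into an alert state with a 2D alarm sound.
; On activation it commits, applies each EffectData entry as a set-by-caller gameplay effect on the owner, stores the handles, and starts the sound.
; It stays active until an Ability.Action.Alert.Stop gameplay event ends it.
; On end it stops the sound and removes every stored effect.
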(event Ability|EventActivateAbility
  (Ability|CommitAbility)
  (CallFunction|ApplyEffect)
  (bind _returnvalue (Audio|SpawnSound2D "/Game/Game/Sounds/Alart.Alart" 1.0 1.0 0.0 0))
  (Variables|Default|SetSound _returnvalue)
  (Ability|Tasks|WaitGameplayEvent "(TagName=\"Ability.Action.Alert.Stop\")" 0
    (:EventReceived
      (Ability|EndAbility))))

(event Ability|EventOnEndAbility
  (params (bWasCancelled :type Boolean))
  (Audio|Components|Audio|Stop (Variables|Default|GetSound))
  (for _array_element (Variables|Default|GetEffectHandle)
    (Ability|RemoveGameplayEffectFromOwnerWithHandle _array_element)))

(fn ApplyEffect
  (for _array_element (Variables|Default|GetEffectData)
    (bind _returnvalue (Ability|GameplayEffect|AssignTagSetbyCallerMagnitude (Ability|MakeOutgoingGameplayEffectSpec (.EffectClass (Utilities|Struct|BreakST_SetbyCollerEffectData _array_element))) (.DataTag (Utilities|Struct|BreakST_SetbyCollerEffectData _array_element)) (.Magnitude (Utilities|Struct|BreakST_SetbyCollerEffectData _array_element))))
    (bind _returnvalue_2 (Ability|ApplyGameplayEffectSpecToOwner _returnvalue))
    (Utilities|Array|Add (Variables|Default|GetEffectHandle) _returnvalue_2))
  (return))