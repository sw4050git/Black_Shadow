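; Gameplay ability for the door key item, used on a key-locked target in the world.
; On activation it commits, gets the owning actor's target through a message call and checks it for the KeyLock tag.
; It sends the unlock message to that target and consumes the selected item through the item manager subsystem only when the call returns false.
; Every path then ends the ability.
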(event Ability|EventActivateAbility
  (bind _returnvalue (Subsystems|GetCPPItemManegerSubsystem))
  (Ability|CommitAbility)
  (bind _targetactor (Class|BPIPlayer|GetTargetActor(Message) (Ability|GetOwningActorfromActorInfo)))
  (Utilities|IsValid _targetactor
    (:Is%20Valid
      (if (Actor|ActorHasTag _targetactor "KeyLock")
        (bind _failed (Class|BPIDoor|DoorUnlock(Message) _targetactor))
        (if _failed
          _
          (else
            (Class|CPPItemManegerSubsystem|ConsumeItem _returnvalue (Variables|/Script/Black_Shadow.CPP_ItemManegerSubsystem|GetSelectedItemData _returnvalue))))
        (Ability|EndAbility)
        (else
          (Ability|EndAbility :!label _label))))
    (:Is%20Not%20Valid
      (goto _label))))

(event Ability|EventOnEndAbility
  (params (bWasCancelled :type Boolean)))