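; Gameplay ability for the lever key item, which unlocks a key-locked lever targeted by its owner.
; On activation it commits, asks the owning actor for its target actor through a message call, and checks that actor for the KeyLockLever tag.
; A valid tagged target receives the lever unlock message, and the ability then ends.
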(event Ability|EventActivateAbility
  (|CallParentFunction)
  (Ability|CommitAbility)
  (bind _targetactor (Class|BPIPlayer|GetTargetActor(Message) (Ability|GetOwningActorfromActorInfo)))
  (Utilities|IsValid _targetactor
    (:Is%20Valid
      (if (Actor|ActorHasTag _targetactor "KeyLockLever")
        (Class|BPILever|LeverUnlock(Message) _targetactor)))
    (:Is%20Not%20Valid
      _))
  (Ability|EndAbility))

(event Ability|EventOnEndAbility
  (params (bWasCancelled :type Boolean))
  (|CallParentFunction bWasCancelled) ; This node is disabled and will not be called.\nDrag off pins to build functionality.
)