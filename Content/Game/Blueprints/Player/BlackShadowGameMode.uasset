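; BlackShadowGameMode is the game mode that manages game-clear and game-over screens and bridges save state with the GameInstance through message calls.
; BeginPlay loads saved memos and items into the C++ memo and item subsystems, then applies settings.
; Save pushes both subsystems' data and temporary actor ID lists back; clearing the game also wipes save data.
; AddTempDestroyedActorID appends to TempActionedActorID, leaving TempDestroyedActorID unfilled here.
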(event Custom|InitMemos
  (bind _memos (Class|BPIGameInstance|GetMemos(Message) (Game|GetGameInstance)))
  (for _array_element _memos
    (Class|CPPMemoManagerSubsystem|AddMemoData (Subsystems|GetCPPMemoManagerSubsystem) _array_element)))

(event Custom|InitItems
  (bind _items (Class|BPIGameInstance|GetItems(Message) (Game|GetGameInstance)))
  (for _array_element _items
    (Class|CPPItemManegerSubsystem|AddItemData (Subsystems|GetCPPItemManegerSubsystem) _array_element)))

(event EventBeginPlay
  (CallFunction|InitMemos)
  (CallFunction|InitItems)
  (Class|BPIGameInstance|ApplySettings(Message) (Game|GetGameInstance)))

(event EventGameOver
  (bind _returnvalue (UserInterface|CreateWidget "/Game/Game/Blueprints/Widget/WB_GameOverUI.WB_GameOverUI_C"))
  (Class|BPIPlayerController|OpenPauseWidget(Message) (Game|GetPlayerController 0) _returnvalue))

(event EventGameClear
  (bind _returnvalue (UserInterface|CreateWidget "/Game/Game/Blueprints/Widget/WB_GameClearUI.WB_GameClearUI_C"))
  (Class|BPIPlayerController|OpenPauseWidget(Message) (Game|GetPlayerController 0) _returnvalue)
  (Class|BPIGameInstance|ClearSaveData(Message) (Game|GetGameInstance)))

(event EventAddTempActionedActorID
  (params (ActionedActorID :type Name :default "None"))
  (Utilities|Set|Add (Variables|Default|GetTempActionedActorID) ActionedActorID))

(event EventAddTempDestroyedActorID
  (params (DestroyedActorID :type Name :default "None"))
  (Utilities|Set|Add (Variables|Default|GetTempActionedActorID) DestroyedActorID))

(event EventSave
  (Class|BPIGameInstance|AddDestroyedActorID(Message) (Game|GetGameInstance) (Variables|Default|GetTempDestroyedActorID))
  (Class|BPIGameInstance|AddActionedActorID(Message) (Game|GetGameInstance) (Variables|Default|GetTempActionedActorID))
  (Class|BPIGameInstance|SetMemos(Message) (Game|GetGameInstance) (Variables|/Script/Black_Shadow.CPP_MemoManagerSubsystem|GetMemos (Subsystems|GetCPPMemoManagerSubsystem)))
  (Class|BPIGameInstance|SetItems(Message) (Game|GetGameInstance) (Variables|/Script/Black_Shadow.CPP_ItemManegerSubsystem|GetItems (Subsystems|GetCPPItemManegerSubsystem))))

(fn ConstructionScript)