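; Game instance for BlackShadow that holds the player's progress and game settings.
; Progress covers items, memos, current and reached phases, and destroyed or actioned actor IDs, all reset by ClearSaveData.
; Settings changes immediately reapply SE volume through a sound mix override and screen resolution through GameUserSettings.
; ClearActionedActorID and ClearDestroyedActorID each empty the opposite set from their name.
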(event Custom|ApplySoundVolume
  ;[1 1 1] Settings
  (Audio|SetSoundMixClassOverride "/Game/Game/Sounds/SCM_Game.SCM_Game" "/Game/Game/Sounds/SoundClass/SC_SE.SC_SE" (Utilities|Struct|BreakST_GameSettings (Variables|Settings|GetGameSettings)) 1.0 0.0 true)
  (Audio|PushSoundMixModifier "/Game/Game/Sounds/SCM_Game.SCM_Game"))

(event Custom|ApplyResolution
  ;[1 1 1] Settings
  (bind _returnvalue (Settings|GetGameUserSettings))
  (Class|GameUserSettings|SetScreenResolution _returnvalue (Utilities|Struct|BreakST_GameSettings (Variables|Settings|GetGameSettings)))
  (Class|GameUserSettings|ApplySettings _returnvalue false))

(event EventSetSoundVolume
  (params (SoundVolume :type Float%20%28double-precision%29))
  ;[1 1 1] Settings
  (Utilities|Struct|SetmembersinST_GameSettings (Variables|Settings|GetGameSettings) SoundVolume)
  (CallFunction|ApplySettings))

(event EventSetResolution
  (params (Resolution :type Int%20Point%20Structure))
  ;[1 1 1] Settings
  (Utilities|Struct|SetmembersinST_GameSettings (Variables|Settings|GetGameSettings) Resolution)
  (CallFunction|ApplySettings))

(event EventAddDestroyedActorID
  (params (ActorID :type Set%20of%20Names))
  ;[1 1 1] ActorManeger
  (Utilities|Set|Union (Variables|ActorManeger|GetDestroyedActorsID) ActorID))

(event EventAddActionedActorID
  (params (ActorID :type Set%20of%20Names))
  ;[1 1 1] ActorManeger
  (Utilities|Set|Union (Variables|ActorManeger|GetActionedActorsID) ActorID))

(event EventSetMemos
  (params (Memo :type Array%20of%20CPP%20Memo%20Data%20Asset%20Object%20References))
  ;[1 1 1] Memo
  (Variables|Memos|SetMemos Memo))

(event EventClearMemos
  ;[1 1 1] Memo
  (Utilities|Array|Clear (Variables|Memos|GetMemos)))

(event EventSetItems
  (params (Item :type Array%20of%20ST%20Item%20Data%20Structures))
  ;[1 1 1] Item
  (Variables|Items|SetItems Item))

(event EventClearItems
  ;[1 1 1] Item
  (Utilities|Array|Clear (Variables|Items|GetItems)))

(event EventSetGameSettings
  (params (GameSettings :type ST%20Game%20Settings%20Structure))
  ;[1 1 1] Settings
  (Variables|Settings|SetGameSettings GameSettings)
  (CallFunction|ApplySettings))

(event EventSetCurrentPhase
  (params (NewPhase :type Gameplay%20Tag%20Structure))
  ;[1 1 1] Phase
  (bind _output_get (Variables|Phase|SetCurrentPhase NewPhase))
  (Utilities|Set|Add (Variables|Phase|GetReachedPhases) _output_get))

(event EventClearActionedActorID
  ;[1 1 1] ActorManeger
  (Utilities|Set|Clear (Variables|ActorManeger|GetDestroyedActorsID)))

(event EventClearDestroyedActorID
  ;[1 1 1] ActorManeger
  (Utilities|Set|Clear (Variables|ActorManeger|GetActionedActorsID)))

(event EventClearSaveData
  ;[1 1 1] General
  (CallFunction|ClearItems)
  (CallFunction|ClearMemos)
  (CallFunction|ClearReachedPhase)
  (CallFunction|ClearActionedActorID)
  (CallFunction|ClearDestroyedActorID))

(event EventClearReachedPhase
  ;[1 1 1] Phase
  (Utilities|Set|Clear (Variables|Phase|GetReachedPhases))
  (Variables|Phase|SetCurrentPhase "(TagName=\"Save.Start\")"))

(event EventApplySettings
  ;[1 1 1] Settings
  (CallFunction|ApplySoundVolume)
  (CallFunction|ApplyResolution))

(fn GetActionedActorsID
  (return (Variables|ActorManeger|GetActionedActorsID)))

(fn GetDestroyedActorsID
  (return (Variables|ActorManeger|GetDestroyedActorsID)))

(fn GetGameSettings
  (return (Variables|Settings|GetGameSettings)))

(fn GetItems
  (return (Variables|Items|GetItems)))

(fn GetMemos
  (return (Variables|Memos|GetMemos)))

(fn GetReachedPhases
  (return (Variables|Phase|GetReachedPhases)))