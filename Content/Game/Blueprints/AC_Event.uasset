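; AC_Event is a component that tracks whether a GUID-identified game event has been executed, with state kept in the game instance.
; Execute and un-execute events set the flag and fire matching event dispatchers, while the check event reads stored state and re-fires the execute dispatcher if set.
; On BeginPlay it binds to GI_BlackShadow's save dispatcher; SaveEventCondition adds or removes the ID from the executed list.
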(event Custom|CheckEventExcuted
  (if (Guid|IsValidGuid (Variables|Default|GetEventID))
    (bind _excuted (Class|BPIGameInstance|CheckEventExcuted(Message) (Game|GetGameInstance) (Variables|Default|GetEventID)))
    (bind _output_get (Variables|Default|SetExcuted _excuted))
    (Development|PrintString (Utilities|String|ToString(Boolean) _output_get))
    (if _output_get
      (Default|CallEDExcuteEvent))))

(event Custom|EventExcute
  (if (Guid|IsValidGuid (Variables|Default|GetEventID))
    (Variables|Default|SetExcuted true)
    (Default|CallEDExcuteEvent)))

(event Custom|EventUnExcute
  (if (Guid|IsValidGuid (Variables|Default|GetEventID))
    (Variables|Default|SetExcuted false)
    (Default|CallEDUnExcuteEvent)))

(event Custom|SaveEventCondition
  (if (Variables|Default|GetExcuted)
    (Class|BPIGameInstance|AddExcutedEventID(Message) (Game|GetGameInstance) (Variables|Default|GetEventID))
    (else
      (Class|BPIGameInstance|RemoveExcutedEventID(Message) (Game|GetGameInstance) (Variables|Default|GetEventID)))))

(event EventBeginPlay
  (Development|PrintString (Guid|ToString(Guid) (Variables|Default|GetEventID)))
  (bind _asgi_black_shadow (Utilities|Casting|CastToGI_BlackShadow (Game|GetGameInstance)))
  (EventDispatchers|BindEventtoEDSave _asgi_black_shadow (EventDispatchers|CreateEvent :!event Custom|SaveEventCondition)))