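; AI controller for the kid NPC that starts its behavior and detects the player.
; On BeginPlay it sets up BB_NpcBase, stores the player pawn as PlayerActor, and runs BT_Npckid.
; AI Perception updates look for actors tagged Player and set Flg_Visible to true when the first last-sensed stimulus succeeds.
; The controller never clears that flag, even when sight of the player is lost.
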(event OnPerceptionUpdated(AIPerception)
  (params (UpdatedActors :type Array%20of%20Actor%20Object%20References))
  ;[1 1 1] AIPerception
  (for _array_element UpdatedActors
    (if (Actor|ActorHasTag _array_element "Player")
      (bind _info (Class|AIPerceptionComponent|GetActorsPerception (Variables|Default|GetAIPerception) _array_element))
      (Class|AIController|UseBlackboard "/Game/Game/Blueprints/Npc/AI/BB_NpcBase.BB_NpcBase")
      (if (.bSuccessfullySensed (Utilities|Struct|BreakAIStimulus (Utilities|Array|Get(acopy) (.LastSensedStimuli (Utilities|Struct|BreakActorPerceptionBlueprintInfo _info)))))
        (AI|Components|Blackboard|SetValueasBool (Variables|Default|GetBlackboard) (Utilities|Name|MakeLiteralName "Flg_Visible") true)))))

(event EventBeginPlay
  ;[1 1 1] BeginPlay
  (Class|AIController|UseBlackboard "/Game/Game/Blueprints/Npc/AI/BB_NpcBase.BB_NpcBase")
  (AI|Components|Blackboard|SetValueasObject (Variables|Default|GetBlackboard) (Utilities|Name|MakeLiteralName "PlayerActor") (Game|Player|GetPlayerPawn 0))
  (AI|RunBehaviorTree "/Game/Game/Blueprints/Npc/AI/BT_Npckid.BT_Npckid"))

(fn ConstructionScript)