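; GI_BlackShadow is the game instance that holds player progress and settings: items, memos, current and reached phases, and IDs of destroyed and actioned actors.
; Simple setter, clear and getter functions manage this state, with phase changes recorded in a reached list and actor IDs merged by union.
; Settings are applied by overriding the SE sound class volume through a sound mix and setting screen resolution through GameUserSettings.
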(event Custom|ApplySoundVolume
  ;[1 1 1] Settings
  (Audio|SetSoundMixClassOverride "/Game/TestGame/Sounds/SCM_Game.SCM_Game" "/Game/TestGame/Sounds/SoundClass/SC_SE.SC_SE" (Utilities|Struct|BreakST_GameSettings (Variables|Settings|GetGameSettings)) 1.0 0.0 true)
  (Audio|PushSoundMixModifier "/Game/TestGame/Sounds/SCM_Game.SCM_Game"))

(event Custom|ApplyResolution
  ;[1 1 1] Settings
  (bind _returnvalue (Settings|GetGameUserSettings))
  (Class|GameUserSettings|SetScreenResolution _returnvalue (Utilities|Struct|BreakST_GameSettings (Variables|Settings|GetGameSettings)))
  (Class|GameUserSettings|ApplySettings _returnvalue false))

(event EventSetSoundVolume
  (params (SoundVolume :type Float%20%28double-precision%29))
  ;[1 1 1] Settings
  (Utilities|Struct|SetmembersinST_GameSettings (Variables|Settings|GetGameSettings) SoundVolume))

(event EventSetResolution
  (params (Resolution :type Int%20Point%20Structure))
  ;[1 1 1] Settings
  (Utilities|Struct|SetmembersinST_GameSettings (Variables|Settings|GetGameSettings) Resolution))

(event EventAddDestroyedActorID
  (params (ActorID :type Set%20of%20Names))
  (Utilities|Set|Union (Variables|Phase|GetDestroyedActorsID) ActorID))

(event EventAddActionedActorID
  (params (ActorID :type Set%20of%20Names))
  (Utilities|Set|Union (Variables|Phase|GetActionedActorsID) ActorID))

(event EventSetGameSettings
  (params (GameSettings :type ST%20Game%20Settings%20Structure))
  ;[1 1 1] Settings
  (Variables|Settings|SetGameSettings GameSettings))

(event EventSetCurrentPhase
  (params (NewPhase :type Gameplay%20Tag%20Structure))
  ;[1 1 1] Phase
  (bind _output_get (Variables|Phase|SetCurrentPhase NewPhase))
  (Utilities|Set|Add (Variables|Phase|GetReachedPhases) _output_get))

(event EventSetItems
  (params (Item :type Array%20of%20ST%20Item%20Structures))
  ;[1 1 1] Item
  (Variables|Default|SetItems Item))

(event EventClearItems
  ;[1 1 1] Item
  (Utilities|Array|Clear (Variables|Default|GetItems)))

(event EventSetMemos
  (params (Memo :type Array%20of%20ST%20Memo%20Structures))
  ;[1 1 1] Memo
  (Variables|Default|SetMemos Memo))

(event EventClearMemos
  ;[1 1 1] Memo
  (Utilities|Array|Clear (Variables|Default|GetMemos)))

(event EventClearReachedPhase
  ;[1 1 1] Phase
  (Utilities|Set|Clear (Variables|Phase|GetReachedPhases))
  (Variables|Phase|SetCurrentPhase "(TagName=\"Save.Start\")"))

(event EventApplySettings
  ;[1 1 1] Settings
  (CallFunction|ApplySoundVolume)
  (CallFunction|ApplyResolution))

(fn GetActionedActorsID
  (return (Variables|Phase|GetActionedActorsID)))

(fn GetDestroyedActorsID
  (return (Variables|Phase|GetDestroyedActorsID)))

(fn GetGameSettings
  (return (Variables|Settings|GetGameSettings)))

(fn GetItems
  (return (Variables|Default|GetItems)))

(fn GetMemos
  (return (Variables|Default|GetMemos)))