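; First-person player character for a stealth game with hiding, peeping, alerts and game over, built on the Gameplay Ability System.
; Startup grants default abilities, a heart-rate effect and the HUD; actions activate abilities by tag and mostly stop them with gameplay events.
; Tick traces from the camera for interactable gimmicks to update the HUD and reports attribute-ranged noise.
; Peep and Hide toggle view-target blends, while death turns the camera before game over.
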(event Custom|SearchTargetGimmick
  (bind _firstpersoncamera (Variables|MyCharacter|GetFirstPersonCamera))
  (bind _returnvalue (Transformation|GetWorldLocation _firstpersoncamera))
  ;[1 1 1] SeachTargetGimmick
  (bind _outhit (Collision|LineTraceByChannel _returnvalue (+ _returnvalue (* (Math|Vector|GetForwardVector (Transformation|GetWorldRotation (Variables|MyCharacter|GetFirstPersonCamera))) 4e+02)) "TraceTypeQuery1" false 0 "None"))
  (Variables|Target|SetTargetActor (.HitActor (Collision|BreakHitResult _outhit)))
  (bind _commandmessage (Class|BPIObject|GetCommandMessage(Message) (Variables|Target|GetTargetActor) self))
  (Class|BPIPlayWidget|SetCommandMessage(Message) (Variables|Widget|GetPlayWidget) _commandmessage)
  (Class|BPIPlayWidget|SetClosshair(Message) (Variables|Widget|GetPlayWidget) (Utilities|IsValid (Variables|Target|GetTargetActor))))

(event Custom|AlertTimer
  ;[1 1 1] Action
  ;;[1 1 1] Alert
  (Ability|SendGameplayEventtoActor self "(TagName=\"Ability.Action.Alert.Stop\")")
  (Utilities|FlowControl|DoOnce false) ; enters at Reset
)

(event Custom|GiveDefaultAbility
  ;[1 1 1] GiveDefaultAbility
  (for _array_element (Variables|Ability|GetDefaultAbilitys)
    (GameplayAbilities|GiveAbility (Variables|Default|GetAbilitySystem) _array_element 0 -1)))

(event Custom|InitStatus
  ;[1 1 1] InitStatus
  (|SetDefaltWalkSpeed
    (:out
      (CallFunction|GiveDefaultAbility)
      (GameplayEffects|ApplyGameplayEffectSpecToSelf (Variables|Default|GetAbilitySystem) (GameplayEffects|MakeOutgoingSpec :self (Variables|Default|GetAbilitySystem) :GameplayEffectClass "/Game/TestGame/Blueprints/GameplayEffect/GE_IncreaseHeartRate.GE_IncreaseHeartRate_C")))))

(event Custom|SetPlayWidget
  ;[1 1 1] SetPlayWidget
  (bind _returnvalue (UserInterface|CreateWidget "/Game/TestGame/Blueprints/Widget/WB_Play.WB_Play_C"))
  (bind _output_get (Variables|Widget|SetPlayWidget _returnvalue))
  (UserInterface|Viewport|AddtoViewport _output_get 0))

(event Input|EnhancedActionEvents|EnhancedInputActionIA_Action_UseItem
  (params (ActionValue :type Boolean) (ElapsedSeconds :type Float%20%28double-precision%29) (TriggeredSeconds :type Float%20%28double-precision%29) (InputAction :type Input%20Action%20Object%20Reference :default "/Game/TestGame/Input/Actions/IA_Action_UseItem.IA_Action_UseItem"))
  ;[1 1 1] Action
  ;;[1 1 1] UseItem
  (bind _returnvalue (GameplayAbilities|GiveAbility (Variables|Default|GetAbilitySystem) (Variables|/Script/Black_Shadow.CPP_ItemDataAsset|GetItemAbility (Variables|/Script/Black_Shadow.CPP_ItemManegerSubsystem|GetSelectedItemData (Subsystems|GetCPPItemManegerSubsystem))) 0 -1))
  (Class|AbilitySystemComponent|TryActivateAbility (Variables|Default|GetAbilitySystem) _returnvalue true)
  (GameplayAbilities|ClearAbility (Variables|Default|GetAbilitySystem) _returnvalue))

(event EventDead
  (params (Direction :type Vector :default "0, 0, 0"))
  ;[1 1 1] Action
  ;;[1 1 1] Dead
  (Input|DisableInput (Game|GetPlayerController 0))
  (bind _newtrack_0 (Timeline|TL_GameOverCamera Play)
    (:Update
      (Pawn|SetControlRotation (Pawn|GetController) (Math|Rotator|Lerp(Rotator) (Pawn|GetControlRotation :!class /Script/Engine.Pawn) (|GetTargetRotator Direction) _newtrack_0 true)))
    (:Finished
      (Class|BPIGameMode|GameOver(Message) (Game|GetGameMode)))))

(event EventStopRun
  ;[1 1 1] Action
  ;;[1 1 1] Run
  (Ability|SendGameplayEventtoActor self "(TagName=\"Ability.Action.Run.Stop\")"))

(event EventBreath
  ;[1 1 1] Action
  ;;[1 1 1] Deep Breath
  (Abilities|TryActivateAbilitiesbyTag (Variables|Default|GetAbilitySystem) (GameplayTags|MakeLiteralGameplayTagContainer "(GameplayTags=((TagName=\"Ability.Action.Breath\")))") true))

(event EventPeep
  (params (Caller :type Actor%20Object%20Reference))
  ;[1 1 1] Action
  ;;[1 1 1] Peep
  (bind _isa (Utilities|FlowControl|FlipFlop)
    (:A
      (CallFunction|StartPeep))
    (:B
      (CallFunction|FInishPeep)))
  (Game|Player|SetViewTargetwithBlend (Game|GetPlayerController 0) (select _isa Caller self) 0.4 "VTBlend_Linear" 0.0 false))

(event EventHide
  (params (Caller :type Actor%20Object%20Reference))
  ;[1 1 1] Action
  ;;[1 1 1] Hide
  (bind _isa (Utilities|FlowControl|FlipFlop)
    (:A
      (CallFunction|StartHide))
    (:B
      (CallFunction|FinishHide)))
  (Game|Player|SetViewTargetwithBlend (Game|GetPlayerController 0) (select _isa Caller self) 0.5 "VTBlend_Linear" 0.0 true))

(event EventStopBreath
  ;[1 1 1] Action
  ;;[1 1 1] Deep Breath
  (Ability|SendGameplayEventtoActor self "(TagName=\"Ability.Action.Breath\")"))

(event EventInteract
  ;[1 1 1] Action
  ;;[1 1 1] Interact
  (Class|BPIObject|Interact(Message) (Variables|Target|GetTargetActor) self))

(event EventTick
  (params (DeltaSeconds :type Float%20%28single-precision%29))
  ;[1 1 1] Tick
  (CallFunction|SearchTargetGimmick)
  (|ReportNoize))

(event EventStartMove
  ;[1 1 1] Action
  ;;[1 1 1] Move
  (Ability|GameplayEffect|AddLooseGameplayTags self (GameplayTags|MakeLiteralGameplayTagContainer "(GameplayTags=((TagName=\"Ability.State.Moving\")))")))

(event EventBeginPlay
  ;[1 1 1] BeginPlay
  (CallFunction|InitStatus)
  (CallFunction|GiveDefaultAbility)
  (CallFunction|SetPlayWidget)
  (Development|ExecuteConsoleCommand "t.MaxFPS 60" 0))

(event EventStopMove
  ;[1 1 1] Action
  ;;[1 1 1] Move
  (Ability|GameplayEffect|RemoveLooseGameplayTags self (GameplayTags|MakeLiteralGameplayTagContainer "(GameplayTags=((TagName=\"Ability.State.Moving\")))"))
  (Ability|SendGameplayEventtoActor self "(TagName=\"Ability.Action.Run.Stop\")"))

(event EventAlert
  ;[1 1 1] Action
  ;;[1 1 1] Alert
  (if (Utilities|Time|IsValidTimerHandle (Variables|Timer|GetTimer))
    (Utilities|Time|ClearandInvalidateTimerbyHandle (Variables|Timer|GetTimer)))
  (bind _returnvalue (Utilities|Time|SetTimerbyEvent (delegate Custom|AlertTimer) 1e+01))
  (Variables|Timer|SetTimer _returnvalue)
  (Utilities|FlowControl|DoOnce false
    (:Completed
      (Abilities|TryActivateAbilitiesbyTag (Variables|Default|GetAbilitySystem) (GameplayTags|MakeLiteralGameplayTagContainer "(GameplayTags=((TagName=\"Ability.Action.Alert\")))") true))))

(event EventSetWalkSpeed
  (params (speed :type Float%20%28single-precision%29))
  ;[1 1 1] SetWalkSpeed
  (Variables|/Script/Engine.CharacterMovementComponent|SetMaxWalkSpeed (Variables|Character|GetCharacterMovement) speed))

(event EventRun
  ;[1 1 1] Action
  ;;[1 1 1] Run
  (Abilities|TryActivateAbilitiesbyTag (Variables|Default|GetAbilitySystem) (GameplayTags|MakeLiteralGameplayTagContainer "(GameplayTags=((TagName=\"Ability.Action.Run\")))") true))

(fn ConstructionScript)

(fn StartPeep
  (Abilities|TryActivateAbilitiesbyTag (Variables|Default|GetAbilitySystem) (GameplayTags|MakeLiteralGameplayTagContainer "(GameplayTags=((TagName=\"Ability.Action.Peep\")))") true))

(fn FInishPeep
  (Ability|SendGameplayEventtoActor self "(TagName=\"Ability.Action.Peep.Finish\")"))

(fn StartHide
  (Rendering|Components|Light|SetIntensity (Variables|Default|GetPointLight) 0.0)
  (Abilities|TryActivateAbilitiesbyTag (Variables|Default|GetAbilitySystem) (GameplayTags|MakeLiteralGameplayTagContainer "(GameplayTags=((TagName=\"Ability.Action.Hide\")))") true))

(fn FinishHide
  (Rendering|Components|Light|SetIntensity (Variables|Default|GetPointLight) 2e+03)
  (Ability|SendGameplayEventtoActor self "(TagName=\"Ability.Action.Hide.Finish\")"))

(fn GetCameraForwardVector
  (return (Math|Vector|GetForwardVector (Variables|MyCharacter|GetFirstPersonCamera))))

(fn GetHeartRate
  (return (.ReturnValue (Ability|Attribute|GetFloatAttributefromAbilitySystemComponent (Variables|Default|GetAbilitySystem) "(AttributeName=\"HeartRate\",Attribute=/Script/Black_Shadow.CPP_PlayerCharacterAttributeSet:HeartRate,AttributeOwner=\"/Script/CoreUObject.Class'/Script/Black_Shadow.CPP_PlayerCharacterAttributeSet'\")"))))

(fn GetPlayWidget
  (return (Variables|Widget|GetPlayWidget)))

(fn GetTargetActor
  (return (Variables|Target|GetTargetActor)))