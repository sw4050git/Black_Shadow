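; Player controller that routes Enhanced Input to the controlled pawn and manages switching between gameplay and the pause menu.
; Move and look apply directly, gated by IsMovable and IsCameraFixed, while run, breath, interact and move start/stop go to the pawn as messages.
; Item selection goes to a play widget fetched from the pawn.
; Opening or closing the menu toggles widget display, input mode, cursor and game pause.
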(event Custom|SetMenuWidget
  (bind _returnvalue (UserInterface|CreateWidget "/Game/TestGame/Blueprints/Widget/WB_Menu.WB_Menu_C"))
  (Variables|Default|SetMenuWidget _returnvalue))

(event Custom|AddInputMapping
  (bind _self self)
  (bind _returnvalue (PlayerController|LocalPlayerSubsystems|GetEnhancedInputLocalPlayerSubsystem _self))
  (Utilities|IsValid _returnvalue
    (:Is%20Valid
      (Input|AddMappingContext _returnvalue "/Game/TestGame/Input/IMC_Action.IMC_Action" 0 "(bIgnoreAllPressedKeysUntilRelease=True,bForceImmediately=False,bNotifyUserSettings=False)"))))

(event Input|EnhancedActionEvents|EnhancedInputActionIA_Action_Move
  (params (ActionValue :type Vector%202D%20Structure) (ElapsedSeconds :type Float%20%28double-precision%29) (TriggeredSeconds :type Float%20%28double-precision%29) (InputAction :type Input%20Action%20Object%20Reference :default "/Game/TestGame/Input/Actions/IA_Action_Move.IA_Action_Move"))
  (bind _returnvalue (Pawn|GetControlledPawn))
  (bind _returnvalue_2 (Pawn|GetControlledPawn))
  (:Triggered
    (if (|IsMovable)
      (Pawn|Input|AddMovementInput _returnvalue (Transformation|GetActorRightVector _returnvalue) (.x ActionValue) false)
      (Pawn|Input|AddMovementInput _returnvalue_2 (Transformation|GetActorForwardVector _returnvalue_2) (.y ActionValue) false)
      (Utilities|FlowControl|DoOnce false :!label _label
        (:Completed
          (Class|BPIPlayer|StartMove(Message) (Pawn|GetControlledPawn))))
      (else
        (Class|BPIPlayer|StopMove(Message) (Pawn|GetControlledPawn) :!label _label_2)
        (goto _label Reset))))
  (:Canceled
    (goto _label_2))
  (:Completed
    (goto _label_2)))

(event Input|EnhancedActionEvents|EnhancedInputActionIA_Action_Run
  (params (ActionValue :type Boolean) (ElapsedSeconds :type Float%20%28double-precision%29) (TriggeredSeconds :type Float%20%28double-precision%29) (InputAction :type Input%20Action%20Object%20Reference :default "/Game/TestGame/Input/Actions/IA_Action_Run.IA_Action_Run"))
  (:Triggered
    (Class|BPIPlayer|Run(Message) (Pawn|GetControlledPawn)))
  (:Completed
    (Class|BPIPlayer|StopRun(Message) (Pawn|GetControlledPawn))))

(event Input|EnhancedActionEvents|EnhancedInputActionIA_Action_Look
  (params (ActionValue :type Vector%202D%20Structure) (ElapsedSeconds :type Float%20%28double-precision%29) (TriggeredSeconds :type Float%20%28double-precision%29) (InputAction :type Input%20Action%20Object%20Reference :default "/Game/TestGame/Input/Actions/IA_Action_Look.IA_Action_Look"))
  (if (not (|IsCameraFixed))
    (Pawn|Input|AddControllerYawInput (Pawn|GetControlledPawn) (.x ActionValue))
    (Pawn|Input|AddControllerPitchInput (Pawn|GetControlledPawn) (.y ActionValue))))

(event Input|EnhancedActionEvents|EnhancedInputActionIA_Action_Breath
  (params (ActionValue :type Boolean) (ElapsedSeconds :type Float%20%28double-precision%29) (TriggeredSeconds :type Float%20%28double-precision%29) (InputAction :type Input%20Action%20Object%20Reference :default "/Game/TestGame/Input/Actions/IA_Action_Breath.IA_Action_Breath"))
  (:Triggered
    (Class|BPIPlayer|Breath(Message) (Pawn|GetControlledPawn)))
  (:Completed
    (Class|BPIPlayer|StopBreath(Message) (Pawn|GetControlledPawn))))

(event Input|EnhancedActionEvents|EnhancedInputActionIA_Action_SelectItem
  (params (ActionValue :type Boolean) (ElapsedSeconds :type Float%20%28double-precision%29) (TriggeredSeconds :type Float%20%28double-precision%29) (InputAction :type Input%20Action%20Object%20Reference :default "/Game/TestGame/Input/Actions/IA_Action_SelectItem.IA_Action_SelectItem"))
  (Class|BPIPlayWidget|SelectItem(Message) (Variables|Default|GetPlayWidget) ActionValue))

(event Input|EnhancedActionEvents|EnhancedInputActionIA_Menu_OpenMenu
  (params (ActionValue :type Boolean) (ElapsedSeconds :type Float%20%28double-precision%29) (TriggeredSeconds :type Float%20%28double-precision%29) (InputAction :type Input%20Action%20Object%20Reference :default "/Game/TestGame/Input/Menu/IA_Menu_OpenMenu.IA_Menu_OpenMenu"))
  (CallFunction|OpenPauseWidget (Variables|Default|GetMenuWidget))
  (Class|BPIMenu|Initalize(Message) (Variables|Default|GetMenuWidget)))

(event Input|EnhancedActionEvents|EnhancedInputActionIA_Action_Interact
  (params (ActionValue :type Boolean) (ElapsedSeconds :type Float%20%28double-precision%29) (TriggeredSeconds :type Float%20%28double-precision%29) (InputAction :type Input%20Action%20Object%20Reference :default "/Game/TestGame/Input/Actions/IA_Action_Interact.IA_Action_Interact"))
  (Class|BPIPlayer|Interact(Message) (Pawn|GetControlledPawn)))

(event EventBeginPlay
  (Input|SetInputModeGameOnly self false)
  (Variables|/Script/Engine.PlayerController|SetbShowMouseCursor self false)
  (CallFunction|SetMenuWidget)
  (CallFunction|AddInputMapping)
  (Utilities|FlowControl|DelayUntilNextTick)
  (bind _widget (Class|BPIPlayer|GetPlayWidget(Message) (Pawn|GetControlledPawn)))
  (Variables|Default|SetPlayWidget _widget))

(event EventClosePauseWidget
  (params (CloseWidget :type User%20Widget%20Object%20Reference))
  (Widget|SetVisibility (Variables|Default|GetPlayWidget) "Visible")
  (Widget|RemovefromParent CloseWidget)
  (Input|SetInputModeGameOnly self false)
  (Variables|/Script/Engine.PlayerController|SetbShowMouseCursor self false)
  (Game|SetGamePaused false))

(event EventOpenPauseWidget
  (params (OpenWidget :type User%20Widget%20Object%20Reference))
  (Widget|SetVisibility (Variables|Default|GetPlayWidget) "Collapsed")
  (UserInterface|Viewport|AddtoViewport OpenWidget 0)
  (Input|SetInputModeUIOnly self 0 "DoNotLock" false)
  (Variables|/Script/Engine.PlayerController|SetbShowMouseCursor self true)
  (Game|SetGamePaused true))

(fn ConstructionScript)