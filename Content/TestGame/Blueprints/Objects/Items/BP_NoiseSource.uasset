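; BP_NoiseSource is a timed noisemaker item that reports noise events for AI hearing, then removes itself.
; BeginPlay waits briefly, plays the Buzaa sound at the Body's location, stops it after a fixed time, then destroys the actor following a further delay.
; While the Noizy flag is set during playback, Tick reports noise every frame with itself as instigator, using Loudness as both volume and maximum range.
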(event EventBeginPlay
  (Utilities|FlowControl|Delay 5.0)
  (Variables|Default|SetNoizy true)
  (bind _returnvalue (Audio|SpawnSoundatLocation "/Game/TestGame/Sounds/buzaa.buzaa" (Transformation|GetWorldLocation (Variables|Default|GetBody)) "0, 0, 0" 1.0 1.0 0.0 0 0))
  (Utilities|FlowControl|Delay 1e+01)
  (Audio|Components|Audio|Stop _returnvalue)
  (Variables|Default|SetNoizy false)
  (Utilities|FlowControl|Delay 1e+01)
  (Actor|DestroyActor))

(event EventTick
  (params (DeltaSeconds :type Float%20%28single-precision%29))
  (bind _loudness (Variables|Default|GetLoudness))
  (if (Variables|Default|GetNoizy)
    (Class|AISenseHearing|ReportNoiseEvent (Transformation|GetWorldLocation (Variables|Default|GetBody)) _loudness self _loudness "None")))

(fn ConstructionScript)