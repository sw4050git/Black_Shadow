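; BP_Memo is an interactable memo pickup that shows a readable note with an image to the player.
; On Action it hides the player's message widget, opens a WB_Memo widget with the memo's image and text, pauses the game and switches to UI-only input with the mouse cursor.
; It also adds the title, text and image to the player's memo archive, and supplies its own command prompt text through GetCommandMessage.
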(event EventBeginPlay)

(event Collision|EventActorBeginOverlap
  (params (OtherActor :type Actor%20Object%20Reference)))

(event EventTick
  (params (DeltaSeconds :type Float%20%28single-precision%29)))

(event EventAction
  (params (Player :type Actor%20Object%20Reference))
  (bind _returnvalue (Game|GetPlayerController 0))
  (bind _widget (Class|BPIFPlayer|GetWidget(Message) Player))
  (Widget|SetVisibility _widget "Collapsed")
  (bind _returnvalue_2 (UserInterface|CreateWidget "/Game/TestGame/Blueprints/UI/WB_Memo.WB_Memo_C"))
  (UserInterface|Viewport|AddtoViewport _returnvalue_2 0)
  (Input|SetInputModeUIOnly _returnvalue 0 "DoNotLock")
  (Game|SetGamePaused true)
  (Variables|/Script/Engine.PlayerController|SetbShowMouseCursor _returnvalue true)
  (Class|BPIFWidget|AddItemImage(Message) _returnvalue_2 (Variables|Default|GetImage) 0 "None")
  (Class|BPIFWidget|SetCommandMassage(Message) _returnvalue_2 (Variables|Default|GetMemo))
  (Class|BPIFPlayer|AddMemoArchive(Message) Player (Variables|Default|GetMemoTitle) (Variables|Default|GetMemo) (Variables|Default|GetImage)))

(fn ConstructionScript)

(fn GetCommandMessage
  (params (Player :type Actor%20Object%20Reference))
  (return (Variables|Default|GetCommandMessage)))