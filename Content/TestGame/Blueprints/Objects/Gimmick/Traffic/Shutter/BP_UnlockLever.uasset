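; BP_UnlockLever is an interactable shutter-gimmick lever that stays locked until LeverUnlock is called, then can be activated once.
; Action fires CallUnlock on first activation and sets Japanese command text for locked, activated or already-active states, returned by GetCommandMessage.
; LeverUnlock records the object-name-derived ID in the GameMode's temporary actioned-actor list.
; BeginPlay restores only the unlocked flag from the GameInstance's list, not activation.
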(event EventBeginPlay
  (bind _actionedactorsid (Class|BPIFGameInstance|GetActionedActorsID(Message) (Game|GetGameInstance)))
  (if (Utilities|Set|Contains _actionedactorsid (Variables|Default|GetID))
    (Variables|Default|SetUnlocked true)))

(event EventAction
  (params (Player :type Actor%20Object%20Reference))
  (if (Variables|Default|GetUnlocked)
    (if (Variables|Default|GetActivated)
      (Variables|Default|SetCommandMassage "すでに起動されている")
      (else
        (Variables|Default|SetActivated true)
        (Default|CallUnlock)
        (Variables|Default|SetCommandMassage "起動した")))
    (else
      (Variables|Default|SetCommandMassage "鍵でロックされている"))))

(event EventLeverUnlock
  (Variables|Default|SetUnlocked true)
  (Variables|Default|SetCommandMassage "動かす")
  (Class|BPIFGameMode|AddTempActionedActorID(Message) (Game|GetGameMode) (Variables|Default|GetID)))

(fn ConstructionScript
  (Variables|Default|SetID (Utilities|String|StringToName (Utilities|GetObjectName self))))

(fn GetCommandMessage
  (params (Player :type Actor%20Object%20Reference))
  (return (Variables|Default|GetCommandMassage)))