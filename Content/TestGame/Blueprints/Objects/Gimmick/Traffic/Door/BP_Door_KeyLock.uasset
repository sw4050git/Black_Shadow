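; Key-locked door that the player cannot open until it is unlocked, built as a child of a parent door Blueprint.
; It sets Locked on BeginPlay, and Action then shows a locked message in place of running the parent's open/close action.
; DoorUnlock clears the lock, switches the prompt to "open" and calls ConnectNpcPath, returning false on unlocking and true if already unlocked.
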(event EventBeginPlay
  (|CallParentFunction)
  (Variables|Default|SetLocked true))

(event EventAction
  (params (Player :type Actor%20Object%20Reference))
  (if (Variables|Default|GetLocked)
    (Variables|Default|SetCommandMassage "鍵がかかっている")
    (else
      (|CallParentFunction 0))))

(fn ConstructionScript
  (|CallParentFunction))

(fn DoorUnlock
  (if (Variables|Default|GetLocked)
    (Variables|Default|SetLocked false)
    (Variables|Default|SetCommandMassage "開ける")
    (CallFunction|ConnectNpcPath)
    (return false)
    (else
      (return true))))