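; Base sliding door gimmick that toggles open and closed through an Action event and supplies a matching Japanese command message.
; A FlipFlop drives a timeline forward or backward, lerping the door sideways by a distance derived from its Y scale.
; Overlapping NPC-tagged actors open it unless locked, rechecking after a delay if it was already open.
; ConnectNpcPath links target points R and L both ways, while DoorUnlock just returns false.
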(event OnComponentBeginOverlap(Box1)
  (params (OverlappedComponent :type Primitive%20Component%20Object%20Reference) (OtherActor :type Actor%20Object%20Reference) (OtherComp :type Primitive%20Component%20Object%20Reference) (OtherBodyIndex :type Integer) (bFromSweep :type Boolean) (SweepResult :type Hit%20Result%20Structure%20%28by%20ref%29))
  (if (not (Variables|Default|GetLocked))
    (if (Actor|ActorHasTag OtherActor "Npc")
      (if (Variables|Default|GetOpened)
        (Utilities|FlowControl|Delay 1.0)
        (if (not (Variables|Default|GetOpened))
          (CallFunction|OpenClose))
        (else
          (CallFunction|OpenClose))))))

(event Custom|OpenClose
  (bind _isa (Utilities|FlowControl|FlipFlop)
    (:A
      (Variables|Default|SetOpened _isa) ; ドアの開閉状態の保存
      (Variables|Default|SetCommandMassage "閉める")
      (bind _newtrack_0 (Timeline|Timeline_1 Play)
        (:Update
          (Transformation|SetRelativeLocation (Variables|Default|GetDoor) (Math|Vector|Lerp(Vector) "0, 0, 0" (Variables|Default|GetDoor%20Width) _newtrack_0) false false))))
    (:B
      (Variables|Default|SetOpened _isa) ; ドアの開閉状態の保存
      (Variables|Default|SetCommandMassage "開ける")
      (Timeline|Timeline_1 Reverse))))

(event EventAction
  (params (Player :type Actor%20Object%20Reference))
  (CallFunction|OpenClose))

(event EventBeginPlay
  (Variables|Default|SetDoor%20Width (CallFunction|GetDoorWidth)))

(fn ConstructionScript)

(fn ConnectNpcPath
  (if (and (Utilities|IsValid (Variables|Default|GetTargetPointR)) (Utilities|IsValid (Variables|Default|GetTargetPointL)))
    (Utilities|Array|AddUnique (Variables|/Game/TestGame/Blueprints/Objects/Gimmick/Traffic/TargetPoint/BP_TargetPoint.BP_TargetPoint_C|GetNextTargetPoints (Variables|Default|GetTargetPointL)) (Variables|Default|GetTargetPointR))
    (Utilities|Array|AddUnique (Variables|/Game/TestGame/Blueprints/Objects/Gimmick/Traffic/TargetPoint/BP_TargetPoint.BP_TargetPoint_C|GetNextTargetPoints (Variables|Default|GetTargetPointR)) (Variables|Default|GetTargetPointL))))

(fn GetDoorWidth
  (return (Math|Vector|MakeVector 0.0 (* (.Y (Math|Vector|BreakVector (Variables|/Script/Engine.SceneComponent|GetRelativeScale3D (Variables|Default|GetDoor)))) 1.8e+02) 0.0)))

(fn DoorUnlock
  (return false))

(fn GetCommandMessage
  (params (Player :type Actor%20Object%20Reference))
  (return (Variables|Default|GetCommandMassage)))