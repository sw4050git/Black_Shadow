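; BP_Bed is an interactable bed gimmick that serves as a player hiding spot.
; Action blends the view target between the bed and the player based on the player's hiding state, then passes the Arrow's world location to the player's HideMessage.
; A FlipFlop toggles the prompt returned by GetCommandMessage between "出る" (exit) and "隠れる" (hide), independently of that state.
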(event EventBeginPlay)

(event Collision|EventActorBeginOverlap
  (params (OtherActor :type Actor%20Object%20Reference)))

(event EventTick
  (params (DeltaSeconds :type Float%20%28single-precision%29)))

(event EventAction
  (params (Player :type Actor%20Object%20Reference))
  (bind _hiding (Class|BPIFPlayer|GetHiding(Message) Player))
  (Game|Player|SetViewTargetwithBlend (Game|GetPlayerController 0) (select _hiding Player self) 0.5 "VTBlend_Linear" 0.0 true)
  (Class|BPIFPlayer|Hide(Message) Player (Transformation|GetWorldLocation (Variables|Default|GetArrow)))
  (Utilities|FlowControl|FlipFlop
    (:A
      (Variables|Default|SetCommandMassage "出る"))
    (:B
      (Variables|Default|SetCommandMassage "隠れる"))))

(fn ConstructionScript)

(fn GetCommandMessage
  (params (Player :type Actor%20Object%20Reference))
  (return (Variables|Default|GetCommandMassage)))