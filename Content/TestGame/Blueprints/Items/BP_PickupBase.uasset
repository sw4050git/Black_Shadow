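; Base pickup actor that, on Interact, adds its Item to the item manager subsystem, destroys itself, and supplies a command message to the player.
; Construction derives a persistent ID from the object name.
; One-time pickups register that ID in the GameMode's temporary destroyed-actor list.
; On BeginPlay, it destroys itself if the GameInstance's destroyed-actor list already contains its ID.
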(event EventBeginPlay
  (bind _destroyedactorsid (Class|BPIGameInstance|GetDestroyedActorsID(Message) (Game|GetGameInstance)))
  (if (Utilities|Set|Contains _destroyedactorsid (Variables|Default|GetID))
    (Actor|DestroyActor)))

(event EventInteract
  (params (Player :type Actor%20Object%20Reference))
  (Class|CPPItemManegerSubsystem|AddItemData (Subsystems|GetCPPItemManegerSubsystem) (Variables|Default|GetItem))
  (if (Variables|Default|GetOnlyOnce)
    (Class|BPIGameMode|AddTempDestroyedActorID(Message) (Game|GetGameMode) (Variables|Default|GetID)))
  (Actor|DestroyActor))

(fn ConstructionScript
  (Variables|Default|SetID (Utilities|String|StringToName (Utilities|GetObjectName self))))

(fn GetCommandMessage
  (params (Player :type Actor%20Object%20Reference))
  (return (Variables|Default|GetCommandMassage)))