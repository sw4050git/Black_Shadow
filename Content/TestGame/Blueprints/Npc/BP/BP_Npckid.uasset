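; BP_Npckid is a kid NPC character that turns into an item pickup when the player touches it.
; On overlap with an actor tagged Player, it spawns a BP_PickupBase at its own transform, copies DropItem and ItemNum onto it, then destroys itself.
; An UpdateWalkSpeed event sets its movement speed, and two getters expose its fixed target point and target point set.
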(event EventBeginPlay)

(event EventUpdateWalkSpeed
  (params (NewWalkSpeed :type Float%20%28double-precision%29))
  (Variables|/Script/Engine.CharacterMovementComponent|SetMaxWalkSpeed (Variables|Character|GetCharacterMovement) NewWalkSpeed))

(event EventTick
  (params (DeltaSeconds :type Float%20%28double-precision%29)))

(event Collision|EventActorBeginOverlap
  (params (OtherActor :type Actor%20Object%20Reference))
  (if (Actor|ActorHasTag OtherActor "Player")
    (bind _returnvalue (Game|SpawnActorfromClass "/Game/TestGame/Blueprints/Objects/Items/BP_PickupBase.BP_PickupBase_C" (Transformation|GetActorTransform) "Undefined" 0 0))
    (Variables|/Game/TestGame/Blueprints/Objects/Items/BP_PickupBase.BP_PickupBase_C|SetItemDataAsset _returnvalue (Variables|Default|GetDropItem))
    (Variables|/Game/TestGame/Blueprints/Objects/Items/BP_PickupBase.BP_PickupBase_C|SetNumber _returnvalue (Variables|Default|GetItemNum))
    (Actor|DestroyActor)))

(fn ConstructionScript)

(fn GetFixTargetPoint
  (return (Variables|Default|GetFixTargetPoint)))

(fn GetTargetPoints
  (return (Variables|Default|GetTargetPoints)))