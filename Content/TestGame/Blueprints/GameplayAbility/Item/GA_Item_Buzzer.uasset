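; GA_Item_Buzzer is the gameplay ability for the buzzer item, which launches a noise source from the owning actor.
; On activation it commits, spawns BP_NoiseSource at the owner's transform, then ends immediately.
; The spawn passes in an Impulse built from the owner's camera forward vector, raised upward and scaled to give a lobbed throw.
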(event Ability|EventActivateAbility
  (|CallParentFunction)
  (Ability|CommitAbility)
  (bind _forwardvector (Class|BPIPlayer|GetCameraForwardVector(Message) (Ability|GetOwningActorfromActorInfo)))
  (Game|SpawnActorfromClass "/Game/TestGame/Blueprints/Gimmick/NoizeSource/BP_NoiseSource.BP_NoiseSource_C" (Transformation|GetActorTransform (Ability|GetOwningActorfromActorInfo)) "Undefined" "OverrideRootScale" 0 (* (Math|Vector|MakeVector (.X (Math|Vector|BreakVector _forwardvector)) (.Y (Math|Vector|BreakVector _forwardvector)) (+ (.Z (Math|Vector|BreakVector _forwardvector)) 1.0)) 5e+02) 0)
  (Ability|EndAbility))

(event Ability|EventOnEndAbility
  (params (bWasCancelled :type Boolean))
  (|CallParentFunction bWasCancelled) ; This node is disabled and will not be called.\nDrag off pins to build functionality.
)