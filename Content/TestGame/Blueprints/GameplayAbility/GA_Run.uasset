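; GA_Run is a Gameplay Ability that keeps the owner in a running state through gameplay effects.
; On activation it commits, applies each EffectData entry with a tag-keyed SetByCaller magnitude, and stores the handles.
; It ends when a Run.Stop gameplay event arrives or the Moving state tag is removed.
; Ending the ability removes all stored effects by handle.
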(event Ability|EventActivateAbility
  (Ability|CommitAbility)
  (CallFunction|ApplyEffects)
  (Ability|Tasks|WaitGameplayEvent "(TagName=\"Ability.Action.Run.Stop\")" 0
    (:then
      (Ability|Tasks|WaitGameplayTagRemove "(TagName=\"Ability.State.Moving\")" 0
        (:Removed
          (Ability|EndAbility))))
    (:EventReceived
      (Ability|EndAbility))))

(event Ability|EventOnEndAbility
  (params (bWasCancelled :type Boolean))
  (for _array_element (Variables|Default|GetEffectHandles)
    (Ability|RemoveGameplayEffectFromOwnerWithHandle _array_element)))

(fn ApplyEffects
  (for _array_element (Variables|Default|GetEffectData)
    (bind _returnvalue (Ability|GameplayEffect|AssignTagSetbyCallerMagnitude (Ability|MakeOutgoingGameplayEffectSpec (.EffectClass (Utilities|Struct|BreakST_SetbyCollerEffectData _array_element))) (.DataTag (Utilities|Struct|BreakST_SetbyCollerEffectData _array_element)) (.Magnitude (Utilities|Struct|BreakST_SetbyCollerEffectData _array_element))))
    (bind _returnvalue_2 (Ability|ApplyGameplayEffectSpecToOwner _returnvalue))
    (Utilities|Array|Add (Variables|Default|GetEffectHandles) _returnvalue_2))
  (return))