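; BP_BlockWall is a traffic gimmick actor that supplies a command message to a querying player.
; The construction script derives its ID from the object name.
; Setting a new message also registers that ID with the game mode as a temporarily actioned actor.
; On BeginPlay, it switches to ChangedMessage if the game instance already lists its ID as actioned, restoring its changed state.
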(event EventBeginPlay
  (bind _actionedactorsid (Class|BPIGameInstance|GetActionedActorsID(Message) (Game|GetGameInstance)))
  (if (Utilities|Set|Contains _actionedactorsid (Variables|Default|GetID))
    (CallFunction|SetCommandMessage (Variables|Default|GetChangedMessage))))

(event EventSetCommandMessage
  (params (NewCommandMessage :type Text))
  (Variables|Default|SetCommandMessage NewCommandMessage)
  (Class|BPIGameMode|AddTempActionedActorID(Message) (Game|GetGameMode) (Variables|Default|GetID)))

(fn ConstructionScript
  (Variables|Default|SetID (Utilities|String|StringToName (Utilities|GetObjectName self))))

(fn GetCommandMessage
  (params (Player :type Actor%20Object%20Reference))
  (return (Variables|Default|GetCommandMessage)))