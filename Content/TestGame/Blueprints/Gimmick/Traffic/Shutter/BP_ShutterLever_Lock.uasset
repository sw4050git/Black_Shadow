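; Shutter lever gimmick that stays locked, as if without power, until all of its linked unlock levers are activated.
; On BeginPlay it locks itself and binds Unlock to each lever in UnlockLevers.
; Each unlock event rechecks every lever's Activated state, then clears the lock and updates the Japanese command message once all are on.
; Action shows a power-off message while locked, otherwise toggles the Shutter through OpenClose.
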(event Custom|Unlock
  (Variables|Default|SetUnlockFlag true)
  (for _array_element (Variables|Default|GetUnlockLevers)
    (if (not (Variables|/Game/TestGame/Blueprints/Gimmick/Traffic/Shutter/BP_UnlockLever.BP_UnlockLever_C|GetActivated _array_element))
      (Variables|Default|SetUnlockFlag false)))
  (if (Variables|Default|GetUnlockFlag)
    (Variables|Default|SetLocked false)
    (Variables|Default|SetCommandMassage "動かす")))

(event EventBeginPlay
  (Utilities|FlowControl|Sequence
    (:then_0
      (Variables|Default|SetLocked true)
      (|CallParentFunction))
    (:then_1
      (for _array_element (Variables|Default|GetUnlockLevers)
        (EventDispatchers|BindEventtoUnlock _array_element (delegate Custom|Unlock))))))

(event Collision|EventActorBeginOverlap
  (params (OtherActor :type Actor%20Object%20Reference))
  (|CallParentFunction OtherActor) ; This node is disabled and will not be called.\nDrag off pins to build functionality.
)

(event EventTick
  (params (DeltaSeconds :type Float%20%28single-precision%29))
  (|CallParentFunction DeltaSeconds) ; This node is disabled and will not be called.\nDrag off pins to build functionality.
)

(event EventAction
  (params (Player :type Actor%20Object%20Reference))
  (if (Variables|Default|GetLocked)
    (Variables|Default|SetCommandMassage "電源が切れている")
    (else
      (Default|OpenClose (Variables|Default|GetShutter)))))

(fn ConstructionScript
  (|CallParentFunction))