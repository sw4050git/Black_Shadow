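; BP_Shutter is a traffic gimmick shutter that opens and closes and can reroute NPC paths around its state.
; OpenClose toggles Opened and runs a timeline forward or backward to slide the Cube between OpenLocation and its relative origin.
; With UseNpcPath, closing unlinks TargetPointL and TargetPointR and links them to target points spawned at the side arrows.
; Opening restores the direct link and destroys the spawned points.
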(event Custom|Initialize%20shutter
  (bind _newtrack_0 (Timeline|Timeline_0 SetNewTime)
    (:Update
      (Transformation|SetRelativeLocation (Variables|Default|GetCube) (Math|Vector|Lerp(Vector) (Variables|Default|GetOpenLocation) "0, 0, 0" _newtrack_0) false false))))

(event Custom|SpawnTargetPoint
  (bind _returnvalue (Game|SpawnActorfromClass "/Game/TestGame/Blueprints/Gimmick/Traffic/TargetPoint/BP_TargetPoint.BP_TargetPoint_C" (Transformation|GetWorldTransform (Variables|Default|GetArrowL)) "Undefined" "MultiplyWithRoot" 0 0))
  (Variables|Default|SetTargetPoint_ShuttersideL _returnvalue)
  (bind _returnvalue_2 (Game|SpawnActorfromClass "/Game/TestGame/Blueprints/Gimmick/Traffic/TargetPoint/BP_TargetPoint.BP_TargetPoint_C" (Transformation|GetWorldTransform (Variables|Default|GetArrowR)) "Undefined" "MultiplyWithRoot" 0 0))
  (Variables|Default|SetTargetPoint_ShuttersideR _returnvalue_2))

(event Custom|DestroyTargetPoint
  (Actor|DestroyActor (Variables|Default|GetTargetPoint_ShuttersideL))
  (Actor|DestroyActor (Variables|Default|GetTargetPoint_ShuttersideR)))

(event Custom|SetPath
  (bind _targetpointl (Variables|Default|GetTargetPointL))
  (bind _targetpointr (Variables|Default|GetTargetPointR))
  (bind _targetpoint_shuttersider (Variables|Default|GetTargetPoint_ShuttersideR))
  (bind _targetpointl_2 (Variables|Default|GetTargetPointL))
  (bind _targetpoint_shuttersidel (Variables|Default|GetTargetPoint_ShuttersideL))
  (bind _nexttargetpoints (Variables|/Game/TestGame/Blueprints/Gimmick/Traffic/TargetPoint/BP_TargetPoint.BP_TargetPoint_C|GetNextTargetPoints _targetpointr))
  (bind _nexttargetpoints_2 (Variables|/Game/TestGame/Blueprints/Gimmick/Traffic/TargetPoint/BP_TargetPoint.BP_TargetPoint_C|GetNextTargetPoints _targetpointl_2))
  (if (Variables|Default|GetUseNpcPath)
    (CallFunction|SpawnTargetPoint)
    (Utilities|Array|RemoveItem _nexttargetpoints_2 (Variables|Default|GetTargetPointR))
    (Utilities|Array|AddUnique _nexttargetpoints_2 _targetpoint_shuttersidel)
    (Utilities|Array|AddUnique (Variables|/Game/TestGame/Blueprints/Gimmick/Traffic/TargetPoint/BP_TargetPoint.BP_TargetPoint_C|GetNextTargetPoints _targetpoint_shuttersidel) _targetpointl_2)
    (Utilities|Array|RemoveItem _nexttargetpoints _targetpointl)
    (Utilities|Array|AddUnique _nexttargetpoints _targetpoint_shuttersider)
    (Utilities|Array|AddUnique (Variables|/Game/TestGame/Blueprints/Gimmick/Traffic/TargetPoint/BP_TargetPoint.BP_TargetPoint_C|GetNextTargetPoints _targetpoint_shuttersider) _targetpointl)))

(event Custom|ResetPath
  (bind _targetpointr (Variables|Default|GetTargetPointR))
  (bind _targetpointl (Variables|Default|GetTargetPointL))
  (bind _nexttargetpoints (Variables|/Game/TestGame/Blueprints/Gimmick/Traffic/TargetPoint/BP_TargetPoint.BP_TargetPoint_C|GetNextTargetPoints _targetpointr))
  (bind _nexttargetpoints_2 (Variables|/Game/TestGame/Blueprints/Gimmick/Traffic/TargetPoint/BP_TargetPoint.BP_TargetPoint_C|GetNextTargetPoints _targetpointl))
  (if (Variables|Default|GetUseNpcPath)
    (Utilities|Array|RemoveItem _nexttargetpoints_2 (Variables|Default|GetTargetPoint_ShuttersideL))
    (Utilities|Array|AddUnique _nexttargetpoints_2 (Variables|Default|GetTargetPointR))
    (Utilities|Array|RemoveItem _nexttargetpoints (Variables|Default|GetTargetPoint_ShuttersideR))
    (Utilities|Array|AddUnique _nexttargetpoints (Variables|Default|GetTargetPointL))
    (CallFunction|DestroyTargetPoint)))

(event Custom|OpenClose
  (if (Variables|Default|GetOpened)
    (CallFunction|SetPath)
    (Variables|Default|SetOpened false)
    (bind _newtrack_0 (Timeline|Timeline_0 Play)
      (:Update
        (Transformation|SetRelativeLocation (Variables|Default|GetCube) (Math|Vector|Lerp(Vector) (Variables|Default|GetOpenLocation) "0, 0, 0" _newtrack_0) false false)))
    (else
      (CallFunction|ResetPath)
      (Variables|Default|SetOpened true)
      (Timeline|Timeline_0 Reverse))))

(event EventBeginPlay
  (CallFunction|SetPath)
  (if (Variables|Default|GetOpened)
    (CallFunction|ResetPath))
  (CallFunction|InitializeShutter))

(event Collision|EventActorBeginOverlap
  (params (OtherActor :type Actor%20Object%20Reference)))

(event EventTick
  (params (DeltaSeconds :type Float%20%28single-precision%29)))

(fn ConstructionScript)

(fn GetCommandMessage
  (params (Player :type Actor%20Object%20Reference))
  (return ""))