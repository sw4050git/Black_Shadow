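; One-sided locked door, a child Blueprint that can only be unlocked from one side.
; A 2D dot product of the door's forward vector and the offset to the player picks the side, with negative counting as the unlock side.
; Interacting there unlocks and toggles the door; from the other side, a locked door only sets a "won't open from here" prompt.
; GetCommandMessage shows an "open" prompt on the unlock side while locked.
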(event EventBeginPlay
  (|CallParentFunction))

(event Collision|EventActorBeginOverlap
  (params (OtherActor :type Actor%20Object%20Reference)))

(event EventTick
  (params (DeltaSeconds :type Float%20%28single-precision%29)))

(event EventInteract
  (params (Player :type Actor%20Object%20Reference))
  (if (CallFunction|CheckPlayerExistForward Player)
    (CallFunction|DoorUnlock)
    (CallFunction|OpenClose)
    (elif (Variables|Default|GetLocked)
      (Variables|Default|SetCommandMessage "こちらからは開かない")
      (else
        (CallFunction|OpenClose)))))

(fn ConstructionScript
  (|CallParentFunction))

(fn CheckPlayerExistForward
  (params (Player :type Actor%20Object%20Reference))
  (bind _returnvalue (Transformation|GetActorRotation))
  (bind _returnvalue_2 (Transformation|GetActorLocation Player))
  (bind _returnvalue_3 (Transformation|GetActorLocation))
  (bind _returnvalue_4 (Math|Vector|GetForwardVector _returnvalue))
  (bind (_x _y) (Math|Vector|BreakVector _returnvalue_2))
  (bind (_x_2 _y_2) (Math|Vector|BreakVector _returnvalue_3))
  (bind (_x_3 _y_3) (Math|Vector|BreakVector _returnvalue_4))
  (return (> 0.0 (+ (* (- _x _x_2) _x_3) (* (- _y _y_2) _y_3)))))

(fn DoorUnlock
  (|CallParentFunction)
  (return false))

(fn GetCommandMessage
  (params (Player :type Actor%20Object%20Reference))
  (if (CallFunction|CheckPlayerExistForward Player)
    (if (Variables|Default|GetLocked)
      (bind _output_get (Variables|Default|SetCommandMessage "開ける"))
      (return _output_get)
      (else
        _)))
  (return (Variables|Default|GetCommandMessage)))