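; Key-locked door gimmick, a child Blueprint that adds lock handling on top of inherited door behavior.
; Interact sets a "鍵がかかっている" (it's locked) command message while Locked, and otherwise calls OpenClose.
; DoorUnlock, when Locked, connects the NPC path, runs the parent unlock and returns false.
; It returns true when the door is not locked.
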(event EventBeginPlay
  (|CallParentFunction))

(event EventInteract
  (params (Player :type Actor%20Object%20Reference))
  (if (Variables|Default|GetLocked)
    (Variables|Default|SetCommandMessage "鍵がかかっている")
    (else
      (CallFunction|OpenClose))))

(fn ConstructionScript
  (|CallParentFunction))

(fn DoorUnlock
  (if (Variables|Default|GetLocked)
    (CallFunction|ConnectNpcPath)
    (|CallParentFunction)
    (return false)
    (else
      (return true))))