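; Blueprint function library with an OpenTutorial function that shows a tutorial popup built from the passed tutorial data.
; It collapses the player character's play UI message, creates a WB_Tutorial widget and adds it to the viewport.
; It switches to UI-only input, pauses the game and shows the cursor, then fills the widget's title and tutorials and calls ChangePage to display them.
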(fn OpenTutorial
  (params (TutorialData :type BP%20Tutorial%20Data%20Object%20Reference))
  (bind _returnvalue (Game|GetPlayerController 0))
  (bind _widget (Class|BPIFPlayer|GetPlayUI(Message) (Game|GetPlayerCharacter 0)))
  (Widget|SetVisibility _widget "Collapsed")
  (bind _returnvalue_2 (UserInterface|CreateWidget "/Game/TestGame/Blueprints/UI/WB_Tutorial.WB_Tutorial_C"))
  (Utilities|FlowControl|Sequence
    (:then_0
      (UserInterface|Viewport|AddtoViewport _returnvalue_2 0)
      (Input|SetInputModeUIOnly _returnvalue 0 "DoNotLock" false)
      (Game|SetGamePaused 0 true)
      (Variables|/Script/Engine.PlayerController|SetbShowMouseCursor _returnvalue true))
    (:then_1
      (Variables|/Game/TestGame/Blueprints/UI/WB_Tutorial.WB_Tutorial_C|SetTitleText _returnvalue_2 (Variables|/Game/TestGame/Blueprints/Objects/Gimmick/Tutorial/BP_TutorialData.BP_TutorialData_C|GetTitle TutorialData))
      (Variables|/Game/TestGame/Blueprints/UI/WB_Tutorial.WB_Tutorial_C|SetTutorials _returnvalue_2 (Variables|/Game/TestGame/Blueprints/Objects/Gimmick/Tutorial/BP_TutorialData.BP_TutorialData_C|GetTutorial TutorialData))
      (Default|ChangePage _returnvalue_2))))