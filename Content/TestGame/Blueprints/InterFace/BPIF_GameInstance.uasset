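; BPIF_GameInstance is a Blueprint interface that exposes persistent game state, presumably held by the game instance.
; It declares phase progress calls to set the current phase and read or clear reached phases, plus accessors for collected items and memos.
; Further calls handle game settings, sound volume and resolution, and record IDs of actioned and destroyed actors.
; All functions are signatures only, with logic left to the implementer.
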(fn ClearReachedPhase)

(fn SetCurrentPhase
  (params (NewPhase :type Gameplay%20Tag%20Structure)))

(fn SetSoundVolume
  (params (SoundVolume :type Float%20%28double-precision%29)))

(fn SetGameSettings
  (params (GameSettings :type ST%20Game%20Settings%20Structure)))

(fn GetGameSettings
  (return ""))

(fn SetResolution
  (params (Resolution :type Int%20Point%20Structure))
  (return))

(fn ClearItems)

(fn GetItems
  (return 0))

(fn SetItems
  (params (Item :type Array%20of%20ST%20Item%20Structures)))

(fn GetMemos
  (return 0))

(fn ClearMemos)

(fn SetMemos
  (params (Memo :type Array%20of%20ST%20Memo%20Structures)))

(fn GetReachedPhases)

(fn ApplySettings)

(fn AddActionedActorID
  (params (ActorID :type Set%20of%20Names)))

(fn AddDestroyedActorID
  (params (ActorID :type Set%20of%20Names)))

(fn GetDestroyedActorsID
  (return 0))

(fn GetActionedActorsID
  (return 0))