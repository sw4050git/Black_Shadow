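; BPIF_Player is a Blueprint Interface that defines how other objects communicate with the player.
; It covers state events such as death, clear and save, hide and peep actions triggered by a caller, and item pickup and consumption.
; It also exposes the memo archive, target actor, play UI, camera forward vector and a heart rate value that doubles as a panic rate.
; All functions are empty declarations, leaving behavior to implementers.
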(fn Dead
  (params (Direction :type Vector))
  (return))

(fn Clear)

(fn Hide
  (params (Caller :type Actor%20Object%20Reference))
  (return))

(fn Pickup
  (params (ItemData :type BP%20Item%20Data%20Asset%20Object%20Reference) (Num :type Integer))
  (return false))

(fn ConsumeItem)

(fn GetMemoArchive
  (return 0))

(fn AddMemoArchive
  (params (MemoTitle :type Text) (Memo :type Text) (Image :type Texture%202D%20Object%20Reference)))

(fn GetTargetActor
  (return 0))

(fn GetPlayUI
  (return 0))

(fn GetHeartRate
  (return 0.0))

(fn GetCameraForwardVector
  (return "0, 0, 0"))

(fn SetHeartRate
  (params (NewPanicRate :type Float%20%28double-precision%29)))

(fn Peep
  (params (Caller :type Actor%20Object%20Reference))
  (return))

(fn Save)